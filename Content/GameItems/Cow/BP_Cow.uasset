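; BP_Cow is a cow game item that spawns a Bpp8 actor when a ThirdPersonCharacter enters its Box trigger.
; The overlap prints a debug "Hello", then spawns only while IsPork8Idle is true, using that flag and a Delay as a short cooldown.
; The spawn point is weighted between the cow and the player camera, a quarter of the way toward the camera and raised slightly.
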(event `self.ReceiveBeginPlay`)

(event `self.Box.OnComponentBeginOverlap`
  (params (OverlappedComponent :type "PrimitiveComponent Object Reference") (OtherActor :type "Actor Object Reference") (OtherComp :type "PrimitiveComponent Object Reference") (OtherBodyIndex :type Integer) (bFromSweep :type Boolean) (SweepResult :type "HitResult Structure (by ref)"))
  (cast `/Game/ThirdPersonBP/Blueprints/ThirdPersonCharacter` OtherActor)
  (`KismetSystemLibrary.PrintString` "Hello")
  (if (`self.IsPork8 Idle`)
    (set `self.IsPork8 Idle` false)
    (`|SpawnActorFromClass` "/Game/Movies/Bpp8.Bpp8_C" (`KismetMathLibrary.Conv_VectorToTransform` (`KismetMathLibrary.MakeVector` (.x (/ (+ (`PlayerCameraManager.GetCameraLocation` (`GameplayStatics.GetPlayerCameraManager` 0)) (* (`self.K2_GetActorLocation`) 3)) 4)) (.y (/ (+ (`PlayerCameraManager.GetCameraLocation` (`GameplayStatics.GetPlayerCameraManager` 0)) (* (`self.K2_GetActorLocation`) 3)) 4)) (+ (.z (/ (+ (`PlayerCameraManager.GetCameraLocation` (`GameplayStatics.GetPlayerCameraManager` 0)) (* (`self.K2_GetActorLocation`) 3)) 4)) 70.0))) "Undefined" "OverrideRootScale" null null)
    (`KismetSystemLibrary.Delay` 2.0)
    (set `self.IsPork8 Idle` true)))

(fn `UserConstructionScript`)